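; BP_RoamingTarget is a destructible, AI-controlled target that wanders the navmesh and takes gun and rocket damage.
; From BeginPlay it repeatedly moves to random navigable points, with a random delay of a few seconds between move requests.
; Point damage from BP_PlayerMovement (rifle or pistol) and radial rocket damage both reduce Health and print debug messages.
; At zero Health, both paths share one exit that spawns the CubeCrumble effect and destroys the actor.
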(event `self.ReceiveBeginPlay`
  (bind _randomlocation (`NavigationSystemV1.K2_GetRandomLocationInNavigableRadius` (`self.K2_GetActorLocation`) 9999.0 null null :!label _label))
  (`AITask_MoveTo.AIMoveTo` (`AIBlueprintHelperLibrary.GetAIController` self) _randomlocation null
    (:`then`
      _)
    (:`OnMoveFinished`
      _))
  (`KismetSystemLibrary.Delay` (`KismetMathLibrary.RandomFloatInRange` 2.0 4.0))
  (goto _label))

(event `self.ReceivePointDamage`
  (params (Damage :type "Float (single-precision)") (DamageType :type "DamageType Object Reference") (HitLocation :type "Vector Structure") (HitNormal :type "Vector Structure") (HitComponent :type "PrimitiveComponent Object Reference") (BoneName :type Name) (ShotFromDirection :type "Vector Structure") (InstigatedBy :type "Controller Object Reference") (DamageCauser :type "Actor Object Reference") (HitInfo :type "HitResult Structure (by ref)"))
  ;[1 1 1] Point Damage (Rifle / Pistol)
  (bind _asbp_player_movement (cast `/Game/BluePrint/BP_PlayerMovement` DamageCauser))
  (if (== (`/Game/BluePrint/BP_PlayerMovement.CurrentEquipped` _asbp_player_movement) 1)
    (`KismetSystemLibrary.PrintString` "Rifle Damage Dealt")
    (else
      (`KismetSystemLibrary.PrintString` "Pistol Damage Dealt")))
  (bind _output_get (set `self.Health` (- (`self.Health`) Damage)))
  (`KismetSystemLibrary.PrintString` (`KismetStringLibrary.Conv_DoubleToString` _output_get))
  (if (<= (`self.Health`) 0.0)
    ;[1 1 1] VFX
    (`NiagaraFunctionLibrary.SpawnSystemAtLocation` "/Game/Particles/CubeCrumble.CubeCrumble" (`self.K2_GetActorLocation`) (struct) (2.0 2.0 2.0) :!label _label_2)
    (`self.K2_DestroyActor`)))

(event `self.ReceiveRadialDamage`
  (params (DamageReceived :type "Float (single-precision)") (DamageType :type "DamageType Object Reference") (Origin :type "Vector Structure") (HitInfo :type "HitResult Structure (by ref)") (InstigatedBy :type "Controller Object Reference") (DamageCauser :type "Actor Object Reference"))
  ;[1 1 1] Radial Damage (Rocket)
  (`KismetSystemLibrary.PrintString` "Rocket Damage")
  (bind _output_get (set `self.Health` (- (`self.Health`) DamageReceived)))
  (`KismetSystemLibrary.PrintString` (`KismetStringLibrary.Conv_DoubleToString` _output_get))
  (if (<= (`self.Health`) 0.0)
    (goto _label_2)))

(fn `UserConstructionScript`)