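; Player character Blueprint that handles firing and switching between rifle, pistol and rocket weapons, plus a level-restart key.
; Holding left mouse runs a per-weapon Delay loop, so each shot, including the first, waits before line tracing from raised actor location along camera forward.
; Hits deal point damage for rifle and pistol, while rockets apply radial falloff damage from a raised origin with Niagara explosion and debug spheres.
; Mouse wheel or numpad plus/minus changes the equipped weapon.
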(event `Key|LeftMouseButton`
  (params (Key :type "Key Structure"))
  (bind _outer_radius (`self.Outer Radius`))
  (bind _inner_radius (`self.Inner Radius`))
  (bind _returnvalue (+ (`self.K2_GetActorLocation` (`ActorComponent.GetOwner` (`self.MainCam`))) (0.0 0.0 80.0)))
  ;[1 1 1] Weapon Organise
  (:`Pressed`
    (set `self.Firing` true)
    (if (== (`self.CurrentEquipped`) 1) :!label _label
      (`KismetSystemLibrary.PrintString` "Rifle")
      (`KismetSystemLibrary.Delay` 0.1 :!label _label_2) ; Rifle
      ;[1 1 1] Shoot
      (if (`self.Firing`) :!label _label_3
        (bind (_outhit _returnvalue_2) (`KismetSystemLibrary.LineTraceSingle` :`Start` _returnvalue :`End` (+ _returnvalue (* (`SceneComponent.GetForwardVector` (`self.MainCam`)) (`self.LengthOfEndCast`))) :`TraceChannel` "TraceTypeQuery1" :`DrawDebugType` "ForDuration"))
        (if _returnvalue_2
          ;[1 1 1] Damage Deal
          (if (== (`self.CurrentEquipped`) 1)
            (bind _asbp_player_movement (cast `/Unreal Engine 5/PC/GunTypes/Blueprints/BP_PlayerMovement` (`GameplayStatics.GetPlayerCharacter` 0)))
            (bind (_bblockinghit _binitialoverlap _time _distance _location _impactpoint _normal _impactnormal _physmat _hitactor) (`GameplayStatics.BreakHitResult` _outhit))
            (`GameplayStatics.ApplyPointDamage` _hitactor 20.0 _impactpoint _outhit (`GameplayStatics.GetPlayerController` 0) _asbp_player_movement "/Script/Engine.DamageType") ; Rifle
            (goto _label_2)
            (elif (== (`self.CurrentEquipped`) 2)
              (bind _asbp_player_movement_2 (cast `/Unreal Engine 5/PC/GunTypes/Blueprints/BP_PlayerMovement` (`GameplayStatics.GetPlayerCharacter` 0)))
              (`GameplayStatics.ApplyPointDamage` _hitactor 35.0 _impactpoint _outhit (`GameplayStatics.GetPlayerController` 0) _asbp_player_movement_2 "/Script/Engine.DamageType") ; Pistol
              (`KismetSystemLibrary.Delay` 0.5 :!label _label_4) ; Pistol
              (goto _label_3)
              (elif (== (`self.CurrentEquipped`) 3)
                (bind _asbp_player_movement_3 (cast `/Unreal Engine 5/PC/GunTypes/Blueprints/BP_PlayerMovement` (`GameplayStatics.GetPlayerCharacter` 0)))
                (`GameplayStatics.ApplyRadialDamageWithFalloff` :`BaseDamage` 100.0 :`MinimumDamage` 10.0 :`Origin` (+ _impactpoint (0.0 0.0 200.0)) :`DamageInnerRadius` _inner_radius :`DamageOuterRadius` _outer_radius :`DamageFalloff` 2.0 :`DamageTypeClass` "/Engine/EngineDamageTypes/DmgTypeBP_Environmental.DmgTypeBP_Environmental_C" :`DamageCauser` _asbp_player_movement_3 :`InstigatedByController` (`GameplayStatics.GetPlayerController` 0) :`DamagePreventionChannel` "ECC_Destructible") ; Rocket
                ;[1 1 1] VFX
                (`KismetSystemLibrary.DrawDebugSphere` _impactpoint _inner_radius 28 (struct :`R` 1.0 :`G` 1.0 :`B` 1.0 :`A` 1.0) 5.0 2.0)
                (`KismetSystemLibrary.DrawDebugSphere` _impactpoint _outer_radius 28 (struct :`R` 1.0 :`G` 1.0 :`B` 1.0 :`A` 1.0) 5.0 2.0)
                (`NiagaraFunctionLibrary.SpawnSystemAtLocation` "/Game/Particles/RocketExplosion.RocketExplosion" _impactpoint (struct) (3.0 3.0 3.0))
                (`KismetSystemLibrary.Delay` 1.0 :!label _label_5) ; Rocket
                (goto _label_3)
                (else
                  (goto _label)))))
          (else
            (`KismetSystemLibrary.PrintString` "No Hit")
            (goto _label)))
        (else
          (`KismetSystemLibrary.PrintString` "Firing Is False")))
      (elif (== (`self.CurrentEquipped`) 2)
        (`KismetSystemLibrary.PrintString` "Pistol")
        (goto _label_4)
        (elif (== (`self.CurrentEquipped`) 3)
          (`KismetSystemLibrary.PrintString` "Rocket")
          (goto _label_5)
          (else
            (`KismetSystemLibrary.PrintString` "ERROR, CURRENT EQUIPPED OUT OF BOUNDS"))))))
  (:`Released`
    (set `self.Firing` false)
    (`KismetSystemLibrary.PrintString` "Release")))

(event `Key|Add`
  (params (Key :type "Key Structure"))
  (bind _currentequipped (`self.CurrentEquipped`))
  ;[1 1 1] Change Weapon
  (:`Pressed`
    (if (<= _currentequipped 2) :!label _label_6
      (bind _output_get (set `self.CurrentEquipped` (+ _currentequipped 1)))
      (`KismetSystemLibrary.PrintString` (`KismetStringLibrary.Conv_IntToString` _output_get))
      (else
        (`KismetSystemLibrary.PrintString` "Can't Go Above Three, No Weapon Equipped To 4")))))

(event `Key|MouseScrollUp`
  (params (Key :type "Key Structure"))
  ;[1 1 1] Change Weapon
  (:`Pressed`
    (goto _label_6)))

(event `Key|R`
  (params (Key :type "Key Structure"))
  ;[1 1 1] Restart Level
  (:`Pressed`
    (`GameplayStatics.OpenLevel` "Map")))

(event `Key|Subtract`
  (params (Key :type "Key Structure"))
  (bind _currentequipped (`self.CurrentEquipped`))
  ;[1 1 1] Change Weapon
  (:`Pressed`
    (if (>= _currentequipped 2) :!label _label_7
      (bind _output_get (set `self.CurrentEquipped` (- _currentequipped 1)))
      (`KismetSystemLibrary.PrintString` (`KismetStringLibrary.Conv_IntToString` _output_get))
      (else
        (`KismetSystemLibrary.PrintString` "Can't Go Below One, No Weapon Equipped To 0")))))

(event `Key|MouseScrollDown`
  (params (Key :type "Key Structure"))
  ;[1 1 1] Change Weapon
  (:`Pressed`
    (goto _label_7)))

(fn `UserConstructionScript`)