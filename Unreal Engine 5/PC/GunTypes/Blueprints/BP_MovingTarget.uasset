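; BP_MovingTarget is an AI-moved shooting target that patrols between two tagged location actors until the player damages it.
; Overlap or hit with BP_LocOne or BP_LocTwo flips a flag that Tick reads to reissue AIMoveTo toward the other point.
; Any player damage stops movement and ticking.
; Point (rifle or pistol) and radial (rocket) damage reduce health, spawning a crumble effect and destroying the target at zero.
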(event `self.ReceiveHit`
  (params (MyComp :type "PrimitiveComponent Object Reference") (Other :type "Actor Object Reference") (OtherComp :type "PrimitiveComponent Object Reference") (bSelfMoved :type Boolean) (HitLocation :type "Vector Structure") (HitNormal :type "Vector Structure") (NormalImpulse :type "Vector Structure") (Hit :type "HitResult Structure (by ref)"))
  ;[1 1 1] Detect When Arrived At Location
  (cast `/Game/BluePrint/BP_LocOne` Other
    (:`then`
      (set `self.HitLocOne` true))
    (:`CastFailed`
      (cast `/Game/BluePrint/BP_LocTwo` Other)
      (set `self.HitLocOne` false))))

(event `self.ReceiveBeginPlay`
  ;[1 1 1] BeginPlay (Set Actor Variables)
  (bind _outactors (`GameplayStatics.GetAllActorsWithTag` "LocOne"))
  (set `self.LocOne` (`|GetArrayItem` _outactors))
  (bind _outactors_2 (`GameplayStatics.GetAllActorsWithTag` "LocTwo"))
  (set `self.LocTwo` (`|GetArrayItem` _outactors_2)))

(event `self.ReceivePointDamage`
  (params (Damage :type "Float (single-precision)") (DamageType :type "DamageType Object Reference") (HitLocation :type "Vector Structure") (HitNormal :type "Vector Structure") (HitComponent :type "PrimitiveComponent Object Reference") (BoneName :type Name) (ShotFromDirection :type "Vector Structure") (InstigatedBy :type "Controller Object Reference") (DamageCauser :type "Actor Object Reference") (HitInfo :type "HitResult Structure (by ref)"))
  ;[1 1 1] Point Damage (Rifle / Pistol)
  (bind _asbp_player_movement (cast `/Game/BluePrint/BP_PlayerMovement` DamageCauser))
  (if (== (`/Game/BluePrint/BP_PlayerMovement.CurrentEquipped` _asbp_player_movement) 1)
    (`KismetSystemLibrary.PrintString` "Rifle Damage Dealt")
    (else
      (`KismetSystemLibrary.PrintString` "Pistol Damage Dealt")))
  (bind _output_get (set `self.Health` (- (`self.Health`) Damage)))
  (`KismetSystemLibrary.PrintString` (`KismetStringLibrary.Conv_DoubleToString` _output_get))
  (if (<= (`self.Health`) 0.0)
    ;[1 1 1] VFX
    (`NiagaraFunctionLibrary.SpawnSystemAtLocation` "/Game/Particles/CubeCrumble.CubeCrumble" (`self.K2_GetActorLocation`) (struct) (2.0 2.0 2.0) :!label _label)
    (`self.K2_DestroyActor`)))

(event `self.ReceiveTick`
  (params (DeltaSeconds :type "Float (single-precision)"))
  (bind _loctwo (`self.LocTwo`))
  (bind _locone (`self.LocOne`))
  (if (`self.IsDamaged`)
    (`KismetSystemLibrary.PrintString` "MoveableTarget Taken Damage")
    (`self.SetActorTickEnabled` false)
    (elif (`self.HitLocOne`)
      ;[1 1 1] Move To Loc One
      (`|AIMoveTo` self (`self.K2_GetActorLocation` _loctwo) _loctwo 10.0
        (:`then`
          _)
        (:`OnSuccess`
          _)
        (:`OnFail`
          _))
      (set `self.HitLocOne` true)
      (else
        ;[1 1 1] Move To Loc One
        (`|AIMoveTo` self (`self.K2_GetActorLocation` _locone) _locone 10.0
          (:`then`
            _)
          (:`OnSuccess`
            _)
          (:`OnFail`
            _))
        (set `self.HitLocOne` false)))))

(event `self.ReceiveRadialDamage`
  (params (DamageReceived :type "Float (single-precision)") (DamageType :type "DamageType Object Reference") (Origin :type "Vector Structure") (HitInfo :type "HitResult Structure (by ref)") (InstigatedBy :type "Controller Object Reference") (DamageCauser :type "Actor Object Reference"))
  ;[1 1 1] Radial Damage (Rocket)
  (`KismetSystemLibrary.PrintString` "Rocket Damage")
  (bind _output_get (set `self.Health` (- (`self.Health`) DamageReceived)))
  (`KismetSystemLibrary.PrintString` (`KismetStringLibrary.Conv_DoubleToString` _output_get))
  (if (<= (`self.Health`) 0.0)
    (goto _label)))

(event `self.ReceiveAnyDamage`
  (params (Damage :type "Float (single-precision)") (DamageType :type "DamageType Object Reference") (InstigatedBy :type "Controller Object Reference") (DamageCauser :type "Actor Object Reference"))
  ;[1 1 1] Take Damage, Stops Movement
  (cast `/Game/BluePrint/BP_PlayerMovement` DamageCauser)
  (set `self.IsDamaged` true)
  (`MovementComponent.StopMovementImmediately` (`self.CharacterMovement`)))

(fn `UserConstructionScript`)