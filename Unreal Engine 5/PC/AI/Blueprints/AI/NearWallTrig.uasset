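; NearWallTrig is a trigger actor that gets zombie AI moving again when it stops near a wall.
; Overlap and Tick share one check on the overlap's actor, acting only on a BP_ZombieAI whose IsMoving is false.
; It sets IsMoving, prints a debug message and sends the zombie to a random reachable point within a wide radius.
; IsMoving clears only when the move succeeds.
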(event `self.ReceiveTick`
  (params (DeltaSeconds :type "Float (single-precision)"))
  (bind _asbp_zombie_ai (cast `/Game/Blueprint/AI/BP_ZombieAI` (stale `self.ReceiveActorBeginOverlap` OtherActor) :!label _label))
  (if (not (`/Game/Blueprint/AI/BP_ZombieAI.IsMoving` _asbp_zombie_ai))
    (set `/Game/Blueprint/AI/BP_ZombieAI.IsMoving` true _asbp_zombie_ai)
    ;[1 1 1] Move AI To A Random Location Within A Radius Of 4000 From Itself
    (`KismetSystemLibrary.PrintString` "Zombie AI Stopped Near Wall, Moving Zombie AI Again")
    (`|AIMoveTo` _asbp_zombie_ai (`NavigationSystemV1.K2_GetRandomReachablePointInRadius` (`self.K2_GetActorLocation` _asbp_zombie_ai) 4000.0 null null) null 5.0 true
      (:`then`
        (bind _asbp_zombie_ai_2 (cast `/Game/Blueprint/AI/BP_ZombieAI` _asbp_zombie_ai))
        (set `/Game/Blueprint/AI/BP_ZombieAI.IsMoving` true _asbp_zombie_ai_2))
      (:`OnSuccess`
        (bind _asbp_zombie_ai_3 (cast `/Game/Blueprint/AI/BP_ZombieAI` _asbp_zombie_ai))
        (set `/Game/Blueprint/AI/BP_ZombieAI.IsMoving` false _asbp_zombie_ai_3)))))

(event `self.ReceiveActorBeginOverlap`
  (params (OtherActor :type "Actor Object Reference"))
  (goto _label))

(fn `UserConstructionScript`)