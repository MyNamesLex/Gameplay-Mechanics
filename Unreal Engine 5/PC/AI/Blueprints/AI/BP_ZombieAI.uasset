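; Zombie AI pawn that roams randomly until it spots the player, then chases them.
; On Tick, while the player is unseen, it waits a random few seconds and moves to a random reachable point nearby.
; Pawn sensing starts the chase, and a retriggerable delay clears the seen flag shortly after the last sighting.
; A hit box overlap with the player currently only prints a hit message.
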(event `self.ReceiveTick`
  (params (DeltaSeconds :type "Float (single-precision)"))
  ;[1 1 1] Wait A Random Amount Of Time
  (if (not (`self.CanSeePlayer`))
    (`KismetSystemLibrary.Delay` (`KismetMathLibrary.RandomFloatInRange` 2.0 4.0))
    ;[1 1 1] Move AI To A Random Location Within A Radius Of 4000 From Itself
    (`|AIMoveTo` self (`NavigationSystemV1.K2_GetRandomReachablePointInRadius` (`self.K2_GetActorLocation`) 4000.0 null null) null 5.0 true
      (:`then`
        (set `self.IsMoving` true))
      (:`OnSuccess`
        (set `self.IsMoving` false)))))

(event `self.PawnSensing.OnSeePawn`
  (params (Pawn :type "Pawn Object Reference"))
  (bind _asbp_player_movement (cast `/Game/Blueprint/Player/BP_PlayerMovement` Pawn))
  (`|ExecutionSequence`
    (:`then_0`
      ;[1 1 1] Chase Player As Soon As AI Sees Player
      (set `self.CanSeePlayer` true)
      (`|AIMoveTo` self (0.0 0.0 0.0) _asbp_player_movement))
    (:`then_1`
      (`KismetSystemLibrary.RetriggerableDelay` 3.5) ; How long the AI will remember where the player is
      (set `self.CanSeePlayer` false))))

(event `self.HitBoxForHitPlayerMechanic.OnComponentBeginOverlap`
  (params (OverlappedComponent :type "PrimitiveComponent Object Reference") (OtherActor :type "Actor Object Reference") (OtherComp :type "PrimitiveComponent Object Reference") (OtherBodyIndex :type Integer) (bFromSweep :type Boolean) (SweepResult :type "HitResult Structure (by ref)"))
  (bind _asbp_player_movement (cast `/Game/Blueprint/Player/BP_PlayerMovement` OtherActor))
  (if (`PrimitiveComponent.IsOverlappingActor` (`Character.CapsuleComponent` _asbp_player_movement) self)
    (`KismetSystemLibrary.PrintString` "Enemy AI Hit Player")))

(fn `UserConstructionScript`)